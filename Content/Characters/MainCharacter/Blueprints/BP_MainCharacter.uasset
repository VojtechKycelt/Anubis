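; Main character Blueprint that adds punch and kick hit detection, passive stamina recovery and a jump cooldown through the Gameplay Ability System.
; Hand and foot colliders attach to mesh sockets and send Punch or Kick gameplay events to self, carrying the overlapped actor as target.
; BeginPlay applies an infinite stamina recovery effect.
; Tick timestamps falling to measure time since landing, allowing CanJumpInternal only after the cooldown and without forbidden tags.
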(event `self.ReceiveBeginPlay`
  (bind _mesh (`self.Mesh`))
  (`|ExecutionSequence`
    (:`then_0`
      (`SceneComponent.K2_AttachToComponent` (`self.RightFootCollider`) _mesh "RightFootSocket" "SnapToTarget" "SnapToTarget" "KeepWorld" true)
      (`SceneComponent.K2_AttachToComponent` (`self.RightHandCollider`) _mesh "RightHandSocket" "SnapToTarget" "SnapToTarget" "KeepWorld" true))
    (:`then_1`
      (`AbilitySystemComponent.BP_ApplyGameplayEffectToSelf` :`self` (`self.AbilitySystemComponent`) :`GameplayEffectClass` "/Game/Characters/MainCharacter/Abilities/GE_Recover_Stamina_Infinite.GE_Recover_Stamina_Infinite_C"))))

(event `self.ReceiveTick`
  (params (DeltaSeconds :type "Float (single-precision)"))
  (`parent.ReceiveTick` DeltaSeconds)
  (`self.JumpCooldown`))

(event `self.RightHandCollider.OnComponentBeginOverlap`
  (params (OverlappedComponent :type "PrimitiveComponent Object Reference") (OtherActor :type "Actor Object Reference") (OtherComp :type "PrimitiveComponent Object Reference") (OtherBodyIndex :type Integer) (bFromSweep :type Boolean) (SweepResult :type "HitResult Structure (by ref)"))
  (if (!= OtherActor self)
    (`AbilitySystemBlueprintLibrary.SendGameplayEventToActor` self (struct :`TagName` "Event.Montage.Punch") (make `GameplayEventData` (struct) self OtherActor null null (struct) (struct) (struct) 0.0 (`AbilitySystemBlueprintLibrary.AbilityTargetDataFromActor` OtherActor)))))

(event `self.RightFootCollider.OnComponentBeginOverlap`
  (params (OverlappedComponent :type "PrimitiveComponent Object Reference") (OtherActor :type "Actor Object Reference") (OtherComp :type "PrimitiveComponent Object Reference") (OtherBodyIndex :type Integer) (bFromSweep :type Boolean) (SweepResult :type "HitResult Structure (by ref)"))
  (if (!= OtherActor self)
    (`AbilitySystemBlueprintLibrary.SendGameplayEventToActor` self (struct :`TagName` "Event.Montage.Kick") (make `GameplayEventData` (struct) self OtherActor null null (struct) (struct) (struct) 0.0 (`AbilitySystemBlueprintLibrary.AbilityTargetDataFromActor` OtherActor)))))

(fn `CanJumpInternal`
  (returns (ReturnValue :type Boolean))
  (return (`self.canJumpAgain`)))

(fn `JumpCooldown`
  (bind (_seconds _partialseconds) (`GameplayStatics.GetAccurateRealTime`))
  (bind (_seconds_2 _partialseconds_2) (`GameplayStatics.GetAccurateRealTime`))
  (`|ExecutionSequence`
    (:`then_0`
      (bind _output_get (set `self.IsFalling` (`NavMovementComponent.IsFalling` (`self.CharacterMovement`))))
      (if _output_get
        (set `self.LandedTime` (+ _seconds _partialseconds))))
    (:`then_1`
      (if (and (> (- (+ _seconds_2 _partialseconds_2) (`self.LandedTime`)) (`self.JumpCooldownTime`)) (not (`GameplayTagAssetInterface.HasAnyMatchingGameplayTags` (`self.AbilitySystemComponent`) (`self.ForbiddenTagsContainer`))))
        (set `self.canJumpAgain` true)
        (else
          (set `self.canJumpAgain` false))))))

(fn `UserConstructionScript`
  (`parent.UserConstructionScript`))