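; Mummy character Blueprint that handles hand collider setup and a ragdoll death.
; On BeginPlay it attaches HandCollider to the mesh's left hand socket.
; MyDeathEvent turns on mesh physics, disables capsule collision and launches the body upward and away from the player with a velocity-change impulse, then destroys the actor after a delay.
; An ability system attribute debug print is left unconnected.
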(event `self.ReceiveBeginPlay`
  (`SceneComponent.K2_AttachToComponent` (`self.HandCollider`) (`self.Mesh`) "LeftHandSocket" "SnapToTarget" "KeepRelative" "KeepWorld" true))

(event `self.ReceiveTick`
  (params (DeltaSeconds :type "Float (single-precision)")))

(event `self.MyDeathEvent`
  (bind _mesh (`self.Mesh`))
  (`PrimitiveComponent.SetCollisionEnabled` _mesh "QueryAndPhysics")
  (`PrimitiveComponent.SetSimulatePhysics` _mesh true)
  (`SkeletalMeshComponent.SetPhysicsBlendWeight` _mesh 1.0)
  (`PrimitiveComponent.SetCollisionEnabled` (`self.CapsuleComponent`) "NoCollision")
  (`PrimitiveComponent.AddImpulse` (`self.Mesh`) (+ (* (`KismetMathLibrary.Vector_Normal2D` (`KismetMathLibrary.GetDirectionUnitVector` (`self.K2_GetActorLocation` (`GameplayStatics.GetPlayerCharacter` 0)) (`self.K2_GetActorLocation`))) (5000.0 5000.0 0.0)) (0.0 0.0 10000.0)) "None" true)
  (`KismetSystemLibrary.Delay` 10.0)
  (`self.K2_DestroyActor`))

(fn `UserConstructionScript`)