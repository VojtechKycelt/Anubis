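; BP_LevelEndDoor is a door actor for the end of a level that marks where the player can interact.
; When the player character enters its Box trigger, it shows a hint Text through AnubisHUD and sets CanInteract on BP_MainCharacter.
; Leaving the box hides the hint and clears that flag.
; The Blueprint itself holds no door opening or level transition logic.
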(event `self.Box.OnComponentBeginOverlap`
  (params (OverlappedComponent :type "PrimitiveComponent Object Reference") (OtherActor :type "Actor Object Reference") (OtherComp :type "PrimitiveComponent Object Reference") (OtherBodyIndex :type Integer) (bFromSweep :type Boolean) (SweepResult :type "HitResult Structure (by ref)"))
  (bind _returnvalue (`GameplayStatics.GetPlayerCharacter` 0))
  (if (== OtherActor _returnvalue)
    (bind _asanubis_hud (cast `AnubisHUD` (`PlayerController.GetHUD` (`GameplayStatics.GetPlayerController` 0))))
    (`AnubisHUD.ShowHint` _asanubis_hud (`self.Text`))
    (bind _asbp_main_character (cast `/Game/Characters/MainCharacter/Blueprints/BP_MainCharacter` _returnvalue))
    (set `AnubisUnrealCharacter.bCanInteract` true _asbp_main_character)))

(event `self.Box.OnComponentEndOverlap`
  (params (OverlappedComponent :type "PrimitiveComponent Object Reference") (OtherActor :type "Actor Object Reference") (OtherComp :type "PrimitiveComponent Object Reference") (OtherBodyIndex :type Integer))
  (bind _returnvalue (`GameplayStatics.GetPlayerCharacter` 0))
  (if (== _returnvalue OtherActor)
    (bind _asanubis_hud (cast `AnubisHUD` (`PlayerController.GetHUD` (`GameplayStatics.GetPlayerController` 0))))
    (`AnubisHUD.HideHint` _asanubis_hud)
    (bind _asbp_main_character (cast `/Game/Characters/MainCharacter/Blueprints/BP_MainCharacter` _returnvalue))
    (set `AnubisUnrealCharacter.bCanInteract` false _asbp_main_character)))

(fn `UserConstructionScript`)