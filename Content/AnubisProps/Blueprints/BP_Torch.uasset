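; BP_Torch is a torch prop that makes its point light flicker.
; BeginPlay caches the light's starting intensity as a baseline.
; Tick runs through a short random Delay, which spaces out the updates irregularly, then sets the intensity to a random value within a narrow band around that baseline.
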(event `self.ReceiveBeginPlay`
  (set `self.baseIntensity` (`LightComponentBase.Intensity` (`self.PointLight`))))

(event `self.ReceiveTick`
  (params (DeltaSeconds :type "Float (single-precision)"))
  (bind _baseintensity (`self.baseIntensity`))
  (`KismetSystemLibrary.Delay` (`KismetMathLibrary.RandomFloatInRange` 0.01 0.1))
  (`LightComponent.SetIntensity` (`self.PointLight`) (`KismetMathLibrary.RandomFloatInRange` (- _baseintensity 1.0) (+ _baseintensity 1.0))))

(fn `UserConstructionScript`)